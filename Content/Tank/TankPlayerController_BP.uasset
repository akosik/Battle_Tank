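; Player controller for the tank that manages the crosshair and respawn countdown UI and handles respawning.
; When an aiming component is found, it creates a crosshair widget bound to that component.
; On tank death, it calls the parent handler, then swaps the crosshair for a countdown seeded from RespawnTime.
; The Respawn input, gated on readiness, removes the countdown, spawns a new tank high above the origin, possesses it and returns to playing state.
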(event EventFoundAimingComponent
  (params (AimCompRef :type Tank%20Aiming%20Component%20Object%20Reference))
  ;[1 1 1] Initialize Crosshair UI
  (bind _returnvalue (UserInterface|CreateWidget "/Game/UI/Crosshair.Crosshair_C"))
  (UserInterface|Viewport|AddtoViewport _returnvalue 0)
  (Variables|/Game/UI/Crosshair.Crosshair_C|SetBP%20Aim%20Comp%20Reference _returnvalue AimCompRef))

(event EventOnTankDeath
  ;[1 1 1] Remove Crossahir UI OnTankDeath, Add Respawn Countdown
  (|CallParentFunction)
  (bind _foundwidgets (Widget|GetAllWidgetsOfClass "/Game/UI/Crosshair.Crosshair_C" true))
  (for _array_element _foundwidgets
    (Widget|RemovefromParent _array_element))
  (bind _returnvalue (UserInterface|CreateWidget "/Game/UI/RespawnCountdown.RespawnCountdown_C"))
  (Variables|/Game/UI/RespawnCountdown.RespawnCountdown_C|SetRespawnCountdown _returnvalue (Math|Float|Truncate (Variables|Default|GetRespawnTime)))
  (UserInterface|Viewport|AddtoViewport _returnvalue 0))

(event Input|ActionEvents|InputActionRespawn
  (params (Key :type Key%20Structure :default "AnyKey"))
  ;[1 1 1] Respawn
  (:Pressed
    (bind _returnvalue (Class|TankPlayerController|GetReadytoRespawn (stale _astank_player_controller_bp)))
    (if _returnvalue
      (bind _foundwidgets (Widget|GetAllWidgetsOfClass "/Game/UI/RespawnCountdown.RespawnCountdown_C" true))
      (Widget|RemovefromParent _foundwidgets)
      (bind _returnvalue_2 (Game|SpawnActorfromClass "/Game/Tank/Tank_BP2.Tank_BP2_C" (Math|Transform|MakeTransform "0.000000, 0,10000.000000") "Undefined" 0 0))
      (Class|TankPlayerController|ToggleReadytoRespawn)
      (Pawn|Possess _returnvalue_2)
      (Class|TankPlayerController|ChangetoPlayingState))))

(fn ConstructionScript)