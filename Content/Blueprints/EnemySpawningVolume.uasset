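; Enemy spawner volume that periodically spawns AI tanks at random points inside its box.
; On BeginPlay, each volume sets a looping SpawnEnemy timer on every EnemySpawningVolume in the level, using its own EnemiesPerSecond rate.
; Each tick of that timer counts all TankAIController_BP actors and spawns a Tank_BP while the count is at most MaxEnemies, so the cap is level-wide.
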(event `self.ReceiveBeginPlay`
  ;[1 1 1] SpawnEnemyLoop
  (bind _outactors (`GameplayStatics.GetAllActorsOfClass` "EnemySpawningVolume_C"))
  (for _array_element _outactors
    (`KismetSystemLibrary.K2_SetTimer` _array_element "SpawnEnemy" (/ 1.0 (`self.EnemiesPerSecond`)) true)))

(event `SpawnEnemy`
  (bind _spawnvolume (`self.SpawnVolume`))
  ;[1 1 1] SpawnEnemy
  (bind _outactors (`GameplayStatics.GetAllActorsOfClass` "/Game/Tank/TankAIController_BP.TankAIController_BP_C"))
  (if (<= (`KismetArrayLibrary.Array_Length` _outactors) (`self.MaxEnemies`))
    (`AIBlueprintHelperLibrary.SpawnAIFromClass` "/Game/Tank/Tank_BP.Tank_BP_C" null (`KismetMathLibrary.RandomPointInBoundingBox` (`SceneComponent.K2_GetComponentLocation` _spawnvolume) (`BoxComponent.GetScaledBoxExtent` _spawnvolume)))))

(fn `UserConstructionScript`)